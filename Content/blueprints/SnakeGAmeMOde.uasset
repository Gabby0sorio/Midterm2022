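; Game mode for a Snake game that spawns fruit and handles game over.
; SpawnFruit, called on BeginPlay, places a Fruitz actor at a fixed height and random X/Y around world origin, within 80% of the extents of the first static mesh tagged "floor".
; GameOver shows the GameOver widget, pauses the game and switches to UI-only input with a visible cursor.
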(event `self.ReceiveBeginPlay`
  (`self.SpawnFruit`))

(event `SpawnFruit`
  (bind _outactors (`GameplayStatics.GetAllActorsOfClassWithTag` "/Script/Engine.StaticMeshActor" "floor"))
  (bind (_origin _boxextent) (`self.GetActorBounds` (`|GetArrayItem` _outactors) false false))
  (`|SpawnActorFromClass` "/Game/blueprints/fruitz.fruitz_C" (`KismetMathLibrary.MakeTransform` (`KismetMathLibrary.MakeVector` (`KismetMathLibrary.RandomFloatInRange` (* (.x _boxextent) -0.8) (* (.x _boxextent) 0.8)) (`KismetMathLibrary.RandomFloatInRange` (* (.y _boxextent) -0.8) (* (.y _boxextent) 0.8)) 270.0)) "Undefined" "OverrideRootScale" null null))

(event `GameOver`
  (bind _returnvalue (`|CreateWidget` "/Game/blueprints/GameOver.GameOver_C" (`GameplayStatics.GetPlayerController` 0)))
  (`UserWidget.AddToViewport` _returnvalue 0)
  (`GameplayStatics.SetGamePaused` true)
  (`WidgetBlueprintLibrary.SetInputMode_UIOnlyEx` (`GameplayStatics.GetPlayerController` 0) _returnvalue)
  (set `PlayerController.bShowMouseCursor` true (`GameplayStatics.GetPlayerController` 0)))

(fn `UserConstructionScript`)