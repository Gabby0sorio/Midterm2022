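; Player-controlled snake for a Snake game, with a score widget, mouse yaw input and an Escape-toggled pause menu.
; Each Tick moves the actor one head-mesh width along MoveDir, then shifts every tail segment into its predecessor's previous position.
; Direction inputs are accepted only when the last move had no component on that axis, blocking reversals.
; EatFruit increments the score and spawns a tail segment using the head's mesh.
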(event `self.ReceiveBeginPlay`
  (bind _returnvalue (`StaticMesh.GetBoundingBox` (`StaticMeshComponent.StaticMesh` (`self.Head`))))
  (set `self.stepsize` (- (.x (`.Max` (break `Box` _returnvalue))) (.x (break `Box` _returnvalue))))
  (bind _returnvalue_2 (`|CreateWidget` "/Game/blueprints/wbp_main.wbp_main_C" (`GameplayStatics.GetPlayerController` 0)))
  (bind _output_get (set `self.UI` _returnvalue_2))
  (`UserWidget.AddToViewport` _output_get 0))

(event `InputAction|MoveUp`
  (params (Key :type "Key Structure"))
  (bind _currentmovedir_x (`KismetMathLibrary.BreakVector` (`self.CurrentMoveDir`)))
  (:`Pressed`
    (if (== _currentmovedir_x 0.0)
      (set `self.MoveDir` (1.0 0.0 0.0)))))

(event `self.ReceiveTick`
  (params (DeltaSeconds :type "Float (single-precision)"))
  (set `self.PreviuosItemLocation` (`self.K2_GetActorLocation`))
  (`self.K2_AddActorWorldOffset` (* (`self.MoveDir`) (`self.stepsize`)))
  (set `self.CurrentMoveDir` (- (`self.K2_GetActorLocation`) (`self.PreviuosItemLocation`)))
  (for _array_element (`self.Tails`)
    (bind _output_get (set `self.Tailcurrentlocation` (`self.K2_GetActorLocation` _array_element)))
    (`self.K2_SetActorLocation` _array_element (`self.PreviuosItemLocation`) false false)
    (set `self.PreviuosItemLocation` _output_get)))

(event `addscore`
  (bind _result (`/Engine/EditorBlueprintResources/StandardMacros.IncrementInt` (`self.Score`))
    (:`  `
      (`/Game/blueprints/wbp_main.SetScore` (`self.UI`) _result))))

(event `InputAction|MoveDown`
  (params (Key :type "Key Structure"))
  (bind _currentmovedir_x (`KismetMathLibrary.BreakVector` (`self.CurrentMoveDir`)))
  (:`Pressed`
    (if (== _currentmovedir_x 0.0)
      (set `self.MoveDir` (-1.0 0.0 0.0)))))

(event `InputAction|MoveRight`
  (params (Key :type "Key Structure"))
  (bind (_currentmovedir_x _currentmovedir_y) (`KismetMathLibrary.BreakVector` (`self.CurrentMoveDir`)))
  (:`Pressed`
    (if (== _currentmovedir_y 0.0)
      (set `self.MoveDir` (0.0 1.0 0.0)))))

(event `Key|Escape` :paused true
  (params (Key :type "Key Structure"))
  (bind _returnvalue (`GameplayStatics.GetPlayerController` 0))
  (:`Pressed`
    (`/Engine/EditorBlueprintResources/StandardMacros.FlipFlop`
      (:`A`
        (bind _returnvalue_2 (`|CreateWidget` "/Game/blueprints/pausemenu.pausemenu_C"))
        (`UserWidget.AddToViewport` _returnvalue_2 0)
        (`GameplayStatics.SetGamePaused` true)
        (set `PlayerController.bShowMouseCursor` true _returnvalue))
      (:`B`
        (`Widget.RemoveFromParent` _returnvalue_2)
        (`GameplayStatics.SetGamePaused` false)
        (set `PlayerController.bShowMouseCursor` false _returnvalue)))))

(event `InputAction|Move Left`
  (params (Key :type "Key Structure"))
  (bind (_currentmovedir_x _currentmovedir_y) (`KismetMathLibrary.BreakVector` (`self.CurrentMoveDir`)))
  (:`Pressed`
    (if (== _currentmovedir_y 0.0)
      (set `self.MoveDir` (0.0 -1.0 0.0)))))

(event `AddTail`
  (bind _returnvalue (`|SpawnActorFromClass` "/Game/blueprints/Tail.Tail_C" (`KismetMathLibrary.MakeTransform` (- (`self.K2_GetActorLocation`) (* (`self.MoveDir`) (`self.stepsize`))) (struct) (0.6 0.6 0.6)) "AlwaysSpawn" "OverrideRootScale" null null))
  (`StaticMeshComponent.SetStaticMesh` (`/Game/blueprints/triggerable.Cube` _returnvalue) (`StaticMeshComponent.StaticMesh` (`self.Head`)))
  (`KismetArrayLibrary.Array_Add` (`self.Tails`) _returnvalue))

(event `EatFruit`
  (`self.addscore`)
  (`self.AddTail`))

(event `InputAxis|Turn`
  (params (AxisValue :type "Float (single-precision)"))
  (`self.AddControllerYawInput` (* AxisValue (`self.mousesens`))))

(fn `UserConstructionScript`)